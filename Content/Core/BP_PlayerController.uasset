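; Player controller for a Paper2D bow character with cursor aiming, linking the pawn to itself and creating the HUD on begin play.
; It forwards axis movement, bow fire/release and scope press/release to BP_PlayerCharacter.
; On tick, while the character passes a Drawing or Scouting state check, a cursor visibility trace yaws the sprite toward the mouse and sets AimTarget.
; A refresh event relays UI updates to the HUD.
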(event Custom|e_BeginPlay
  (Utilities|FlowControl|Sequence
    (:then_0
      (bind _asbp_player_character (Utilities|Casting|CastToBP_PlayerCharacter (Pawn|GetControlledPawn))
        (:then
          (bind _output_get (Variables|Default|SetPlayerPawn _asbp_player_character))
          (Variables|/Game/Core/BP_PlayerCharacter.BP_PlayerCharacter_C|SetPlayerController _output_get self))
        (:CastFailed
          (Development|PrintString "NO CONTROLLED PAWN" true true "(R=1.000000,G=0.000000,B=0.039766,A=1.000000)" 99.0))))
    (:then_1
      (bind _returnvalue (UserInterface|CreateWidget "/Game/UI/UI_HUD.UI_HUD_C" self))
      (bind _output_get_2 (Variables|Default|SetHUD _returnvalue))
      (Variables|/Game/UI/UI_HUD.UI_HUD_C|SetPawn _output_get_2 (.Player%20Character (CallFunction|FGetControlledPlayerCharacter)))
      (Utilities|IsValid _output_get_2
        (:Is%20Valid
          (UserInterface|Viewport|AddtoViewport _output_get_2 0))))))

(event Custom|e_TickEvent
  (bind (_player_character _success) (CallFunction|FGetControlledPlayerCharacter))
  (if _success
    (bind _state_match (Default|FStateCheck _player_character false true true))
    (if _state_match
      (CallFunction|FRotatetoMouse))))

(event Custom|e_RefreshUI
  (Default|ERefreshUI (Variables|Default|GetHUD)))

(event EventBeginPlay
  (CallFunction|EBeginPlay))

(event EventTick
  (params (DeltaSeconds :type Float%20%28single-precision%29))
  (CallFunction|ETickEvent))

(event Input|ActionEvents|InputActionBowFire
  (params (Key :type Key%20Structure))
  (bind _player_character (CallFunction|FGetControlledPlayerCharacter))
  (:Pressed
    (Default|EBowFire _player_character))
  (:Released
    (Default|EBowRelease _player_character)))

(event Input|ActionEvents|InputActionScope
  (params (Key :type Key%20Structure))
  (bind _player_character (CallFunction|FGetControlledPlayerCharacter))
  (:Pressed
    (Default|EBeginScout _player_character))
  (:Released
    (Default|EEndScout _player_character "NewEnumerator0")))

(event Input|AxisEvents|InputAxisA_Horizontal
  (params (AxisValue :type Float%20%28single-precision%29))
  (bind (_player_character _success) (CallFunction|FGetControlledPlayerCharacter))
  (if _success
    (Pawn|Input|AddMovementInput _player_character (Math|Vector|GetForwardVector (Math|Rotator|MakeRotator 0.0 (.pitch (Pawn|GetControlRotation _player_character :!class /Script/Engine.Pawn)) 0.0)) AxisValue false)))

(event Input|AxisEvents|InputAxisA_Vertical
  (params (AxisValue :type Float%20%28single-precision%29))
  (bind (_player_character _success) (CallFunction|FGetControlledPlayerCharacter))
  (if _success
    (Pawn|Input|AddMovementInput _player_character (Math|Vector|GetRightVector (Math|Rotator|MakeRotator 0.0 (.pitch (Pawn|GetControlRotation _player_character :!class /Script/Engine.Pawn)) 0.0)) AxisValue false)))

(fn ConstructionScript)

(fn FRotatetoMouse
  (bind (_player_character _success) (CallFunction|FGetControlledPlayerCharacter))
  (bind _hitresult (Game|Player|GetHitResultUnderCursorbyChannel "TraceTypeQuery1" true))
  (bind _playerpawn (Variables|Default|GetPlayerPawn))
  (bind _location (Collision|BreakHitResult _hitresult))
  (Transformation|SetWorldRotation (Variables|/Game/Core/BP_PlayerCharacter.BP_PlayerCharacter_C|GetPaperSprite _playerpawn) (Math|Rotator|MakeRotator 9e+01 0.0 (.yaw (Math|Rotator|FindLookatRotation (Transformation|GetActorLocation _playerpawn) _location))) false false)
  (if _success
    (bind _output_get (Variables|/Game/Core/BP_PlayerCharacter.BP_PlayerCharacter_C|SetAimTarget _player_character _location))
    (Variables|Default|SetAimTarget _output_get)))

(fn FGetControlledPlayerCharacter
  (bind _returnvalue (Pawn|GetControlledPawn))
  (bind (_asbp_player_character _bsuccess) (Utilities|Casting|CastToBP_PlayerCharacter _returnvalue))
  (return _asbp_player_character _bsuccess))