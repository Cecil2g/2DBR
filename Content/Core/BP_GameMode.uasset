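; Game mode for a shrinking play area with deadzones, but every event and the resize entry are unwired, so none of it runs.
; The disconnected logic spawns a 16-square grid from a data table and builds player minimaps.
; A countdown removes marked squares and advances phases, each placing an area selector randomly offset from the remaining squares' average, with some cuts perpendicular to the last.
; The final phase enables encroachment instead.
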(event Custom|e_PhaseIncrement)

(event Custom|e_GameStart)

(event Custom|e_DestroyMarked)

(event Custom|e_RefreshPlayerMinimaps)

(event Custom|e_GameModeMessage
  (params (Message%20In :type Text)))

(event EventBeginPlay)

(event EventTick
  (params (DeltaSeconds :type Float%20%28single-precision%29)))

(fn ConstructionScript)

(fn FSpawnSquare
  (params (Ref%20In :type Integer))
  (bind _gridsize (Variables|Default|GetGridSize))
  (bind _returnvalue (Utilities|GetDataTableRow "/Game/Core/DT_AreaLimitData.DT_AreaLimitData" (Utilities|String|StringToName (Utilities|String|ToString(Integer) Ref%20In)))
    (:then
      (bind _returnvalue_2 (Game|SpawnActorfromClass "/Game/Core/BP_AreaLimit.BP_AreaLimit_C" (Math|Transform|MakeTransform (+ (Math|Vector|MakeVector (* (.xoffset _returnvalue) _gridsize) (* (.yoffset _returnvalue) _gridsize) 0.0) (Math|Vector|MakeVector 0.0 0.0 0.0)) "0, 0, 0" "1,1,1") "Undefined" 0 0))
      (Transformation|SetActorLocation _returnvalue_2 (Math|Vector|MakeVector (- (.x (Transformation|GetActorLocation _returnvalue_2)) 8.0) (- (.y (Transformation|GetActorLocation _returnvalue_2)) 8.0) (.z (Transformation|GetActorLocation _returnvalue_2))) false false)
      (Utilities|Array|Add (Variables|Default|GetAreaLimits) _returnvalue_2))
    (:RowNotFound
      (Development|PrintString "DT NOT FOUND"))))

(fn FGetAverageVector
  (bind _arealimits (Variables|Default|GetAreaLimits))
  (Development|PrintString (Utilities|String|ToString(Integer) (Utilities|Array|Length _arealimits)))
  (for _array_element _arealimits
    (LocalVariables|SetAverageVector (+ (Transformation|GetActorLocation _array_element) (LocalVariables|GetAverageVector)))
    (Math|Integer|IncrementInt (LocalVariables|GetAreaCount)))
  (return (/ (LocalVariables|GetAverageVector) (LocalVariables|GetAreaCount))))

(fn FResize1
  (bind _averagevector_out (CallFunction|FGetAverageVector))
  (bind _dimension (LocalVariables|GetDimension))
  (switch int (Math|Random|RandomIntegerinRange 1 4)
    (:1
      (LocalVariables|SetLocal%20Vector (Math|Vector|MakeVector (+ (.x _averagevector_out) _dimension) (.y _averagevector_out) 0.0))
      (LocalVariables|SetLocal%20Scale "1.500000,3.500000,1.000000" :!label _label)
      (Variables|Default|SetLast%20Reduction "NewEnumerator1"))
    (:2
      (LocalVariables|SetLocal%20Vector (Math|Vector|MakeVector (- (.x _averagevector_out) _dimension) (.y _averagevector_out) 0.0))
      (goto _label))
    (:3
      (LocalVariables|SetLocal%20Vector (Math|Vector|MakeVector (.x _averagevector_out) (+ (.y _averagevector_out) _dimension) 0.0))
      (LocalVariables|SetLocal%20Scale "3.500000,1.500000,1.000000" :!label _label_2)
      (Variables|Default|SetLast%20Reduction "NewEnumerator0"))
    (:4
      (LocalVariables|SetLocal%20Vector (Math|Vector|MakeVector (.x _averagevector_out) (- (.y _averagevector_out) _dimension) 0.0))
      (goto _label_2)))
  (return (LocalVariables|GetLocal%20Vector) (LocalVariables|GetLocal%20Scale)))

(fn FResize2
  (bind _averagevector_out (CallFunction|FGetAverageVector))
  (bind _returnvalue (Math|Random|RandomIntegerinRange 1 2))
  (bind _dimension (LocalVariables|GetDimension))
  (switch Utilities|FlowControl|Switch|SwitchonE_ReductionTypes (Variables|Default|GetLast%20Reduction)
    (:NewEnumerator0
      (switch int _returnvalue
        (:1
          (LocalVariables|SetLocal%20Vector (Math|Vector|MakeVector (+ (.x _averagevector_out) _dimension) (.y _averagevector_out) 0.0)))
        (:2
          (LocalVariables|SetLocal%20Vector (Math|Vector|MakeVector (- (.x _averagevector_out) _dimension) (.y _averagevector_out) 0.0))))
      (LocalVariables|SetLocal%20Scale "1.000000,1.000000,1.000000"))
    (:NewEnumerator1
      (switch int _returnvalue
        (:1
          (LocalVariables|SetLocal%20Vector (Math|Vector|MakeVector (.x _averagevector_out) (+ (.y _averagevector_out) _dimension) 0.0)))
        (:2
          (LocalVariables|SetLocal%20Vector (Math|Vector|MakeVector (.x _averagevector_out) (- (.y _averagevector_out) _dimension) 0.0))))
      (LocalVariables|SetLocal%20Scale "1.000000,1.000000,1.000000")))
  (return (LocalVariables|GetLocal%20Vector) (LocalVariables|GetLocal%20Scale)))

(fn FResize3
  (bind _averagevector_out (CallFunction|FGetAverageVector))
  (bind _dimension (LocalVariables|GetDimension))
  (switch int (Math|Random|RandomIntegerinRange 1 4)
    (:1
      (LocalVariables|SetLocal%20Vector (Math|Vector|MakeVector (+ (.x _averagevector_out) _dimension) (.y _averagevector_out) 0.0))
      (LocalVariables|SetLocal%20Scale "1.000000,1.000000,1.000000" :!label _label)
      (Variables|Default|SetLast%20Reduction "NewEnumerator1"))
    (:2
      (LocalVariables|SetLocal%20Vector (Math|Vector|MakeVector (- (.x _averagevector_out) _dimension) (.y _averagevector_out) 0.0))
      (goto _label))
    (:3
      (LocalVariables|SetLocal%20Vector (Math|Vector|MakeVector (.x _averagevector_out) (+ (.y _averagevector_out) _dimension) 0.0))
      (LocalVariables|SetLocal%20Scale "1.000000,1.000000,1.000000" :!label _label_2)
      (Variables|Default|SetLast%20Reduction "NewEnumerator0"))
    (:4
      (LocalVariables|SetLocal%20Vector (Math|Vector|MakeVector (.x _averagevector_out) (- (.y _averagevector_out) _dimension) 0.0))
      (goto _label_2)))
  (return (LocalVariables|GetLocal%20Vector) (LocalVariables|GetLocal%20Scale)))

(fn FResize4
  (bind _averagevector_out (CallFunction|FGetAverageVector))
  (bind _returnvalue (Math|Random|RandomIntegerinRange 1 2))
  (bind _dimension (LocalVariables|GetDimension))
  (switch Utilities|FlowControl|Switch|SwitchonE_ReductionTypes (Variables|Default|GetLast%20Reduction)
    (:NewEnumerator0
      (switch int _returnvalue
        (:1
          (LocalVariables|SetLocal%20Vector (Math|Vector|MakeVector (+ (.x _averagevector_out) _dimension) (.y _averagevector_out) 0.0)))
        (:2
          (LocalVariables|SetLocal%20Vector (Math|Vector|MakeVector (- (.x _averagevector_out) _dimension) (.y _averagevector_out) 0.0))))
      (LocalVariables|SetLocal%20Scale "0.500000,0.500000,1.000000"))
    (:NewEnumerator1
      (switch int _returnvalue
        (:1
          (LocalVariables|SetLocal%20Vector (Math|Vector|MakeVector (.x _averagevector_out) (+ (.y _averagevector_out) _dimension) 0.0)))
        (:2
          (LocalVariables|SetLocal%20Vector (Math|Vector|MakeVector (.x _averagevector_out) (- (.y _averagevector_out) _dimension) 0.0))))
      (LocalVariables|SetLocal%20Scale "0.500000,0.500000,1.000000")))
  (return (LocalVariables|GetLocal%20Vector) (LocalVariables|GetLocal%20Scale)))

(fn FResizeGameArea
  (params (Selection :type Integer) (Area%20Selector%20In :type Actor%20Object%20Reference)))

(fn FGameModeMessage
  (params (Message%20In :type Text))
  (bind _outactors (Actor|GetAllActorsOfClass "/Game/Core/BP_PlayerController.BP_PlayerController_C"))
  (for _array_element _outactors
    (Default|EHUDGameModeMessage (Variables|/Game/Core/BP_PlayerController.BP_PlayerController_C|GetHUD _array_element) _array_element Message%20In))
  (return))

(fn FMakeMinimap
  (bind _outactors (Actor|GetAllActorsOfClass "/Game/Core/BP_PlayerController.BP_PlayerController_C"))
  (for _array_element _outactors
    (Default|EMakeGridSquares (Variables|/Game/UI/UI_HUD.UI_HUD_C|GetUI_Minimap (Variables|/Game/Core/BP_PlayerController.BP_PlayerController_C|GetHUD _array_element)))))