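; Treasure chest actor that drops a random special arrow pickup the first time the player character overlaps it.
; A random roll picks the smoke, fire or ice row from DT_ArrowTypes.
; It spawns a BP_ArrowPickup at the chest's transform and hands it that row as its ArrowData.
; The chest then sets its Open flag to block repeat drops and swaps the Cube's material.
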(event Custom|e_SpawnLoot
  (CallFunction|FSpawnLoot))

(event EventBeginPlay)

(event Collision|EventActorBeginOverlap
  (params (OtherActor :type Actor%20Object%20Reference))
  (if (not (Variables|Default|GetOpen))
    (if (.bSuccess (Utilities|Casting|CastToBP_PlayerCharacter OtherActor))
      (CallFunction|ESpawnLoot))))

(event EventTick
  (params (DeltaSeconds :type Float%20%28single-precision%29)))

(fn ConstructionScript)

(fn FSpawnLoot
  (switch int (Math|Random|RandomIntegerinRange 1 3)
    (:1
      (bind _returnvalue (Utilities|GetDataTableRow "/Game/Core/DT_ArrowTypes.DT_ArrowTypes" "arrow_smoke")
        (:then
          (LocalVariables|SetLocal_Data _returnvalue))))
    (:2
      (bind _returnvalue_2 (Utilities|GetDataTableRow "/Game/Core/DT_ArrowTypes.DT_ArrowTypes" "arrow_fire")
        (:then
          (LocalVariables|SetLocal_Data _returnvalue_2))))
    (:3
      (bind _returnvalue_3 (Utilities|GetDataTableRow "/Game/Core/DT_ArrowTypes.DT_ArrowTypes" "arrow_ice")
        (:then
          (LocalVariables|SetLocal_Data _returnvalue_3)))))
  (bind _returnvalue_4 (Game|SpawnActorfromClass "/Game/Core/BP_ArrowPickup.BP_ArrowPickup_C" (Transformation|GetActorTransform) "Undefined" 0 0))
  (Variables|/Game/Core/BP_ArrowPickup.BP_ArrowPickup_C|SetArrowData _returnvalue_4 (LocalVariables|GetLocal_Data))
  (Variables|Default|SetOpen true)
  (Rendering|Material|SetMaterial (Variables|Default|GetCube) 0 "/Game/Starter/2D/SpriteMaterial.SpriteMaterial")
  (return))