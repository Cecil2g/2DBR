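; BP_Arrow is an arrow actor that applies damage to whatever its Box component hits.
; On BeginPlay the box ignores its owner when moving, and Tick destroys the arrow once LifeTime is at or below zero.
; Hits credit the instigator's controller with the arrow as causer, but do not destroy it, as that destroy call is unconnected.
; Damage has an empty OnRep function.
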(event OnComponentHit(Box)
  (params (HitComponent :type Primitive%20Component%20Object%20Reference) (OtherActor :type Actor%20Object%20Reference) (OtherComp :type Primitive%20Component%20Object%20Reference) (NormalImpulse :type Vector :default "0, 0, 0") (Hit :type Hit%20Result%20Structure%20%28by%20ref%29))
  (Game|Damage|ApplyDamage OtherActor (Variables|Default|GetDamage) (Game|GetInstigatorController) self))

(event EventBeginPlay
  (bind _returnvalue (Components|GetOwner))
  (Development|PrintString (Utilities|String|Append "Arrow is ignoring actor: " (Utilities|GetDisplayName _returnvalue)))
  (Collision|IgnoreActorwhenMoving (Variables|Default|GetBox) _returnvalue true))

(event Collision|EventActorBeginOverlap
  (params (OtherActor :type Actor%20Object%20Reference)))

(event EventTick
  (params (DeltaSeconds :type Float%20%28single-precision%29))
  (CallFunction|-=Float (Variables|Default|GetLifeTime) DeltaSeconds)
  (if (<= (Variables|Default|GetLifeTime) 0.0)
    (Actor|DestroyActor)))

(fn ConstructionScript)

(fn OnRepDamage)