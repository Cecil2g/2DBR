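; Arrow pickup actor that adds its arrow type and count to a player character's arrow inventory on overlap.
; FLootArrow ignores non-player actors and the pickup's own Instigator, then increases the count of the entry matching by name or adds a new one, and destroys the pickup.
; Tick pins the actor's world Z to a fixed height.
; The HUD refresh call is left unwired.
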(event EventBeginPlay)

(event Collision|EventActorBeginOverlap
  (params (OtherActor :type Actor%20Object%20Reference))
  (CallFunction|FLootArrow OtherActor))

(event EventTick
  (params (DeltaSeconds :type Float%20%28single-precision%29))
  (bind _returnvalue (Transformation|GetActorLocation))
  (Transformation|SetActorLocation (Math|Vector|MakeVector (.x _returnvalue) (.y _returnvalue) 33.0) false false))

(fn ConstructionScript)

(fn FLootArrow
  (params (Object :type Object%20Object%20Reference))
  (bind _arrowdata (Variables|Default|GetArrowData))
  (bind _asbp_player_character (Utilities|Casting|CastToBP_PlayerCharacter Object)
    (:then
      (if (== (Variables|Actor|GetInstigator) _asbp_player_character)
        _
        (else
          (for (_ _array_index) (Variables|/Game/Core/BP_PlayerCharacter.BP_PlayerCharacter_C|GetArrowArray _asbp_player_character)
            (if (Utilities|Name|Equal(Name) (.name (Utilities|Array|Get(acopy) (Variables|/Game/Core/BP_PlayerCharacter.BP_PlayerCharacter_C|GetArrowArray _asbp_player_character) _array_index)) (.name _arrowdata))
              (for _index (range 1 (.count _arrowdata))
                (Math|Integer|IncrementInt (.count (Utilities|Array|Get(acopy) (Variables|/Game/Core/BP_PlayerCharacter.BP_PlayerCharacter_C|GetArrowArray _asbp_player_character) _array_index))))
              (Actor|DestroyActor)
              (return)))
          (Utilities|Array|AddUnique (Variables|/Game/Core/BP_PlayerCharacter.BP_PlayerCharacter_C|GetArrowArray _asbp_player_character) (Variables|Default|GetArrowData))
          (Actor|DestroyActor)
          (return))))
    (:CastFailed
      _))
  (return))