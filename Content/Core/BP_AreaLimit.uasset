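; BP_AreaLimit is a cube actor, apparently an area boundary, that can shrink away and remove itself.
; While Encroachment is set, Tick reduces the cube's X and Y scale by a fixed, frame-rate-dependent step, holds Z at one, and destroys the actor near zero.
; e_MarkSquare only sets a Destroy flag, which nothing here reads.
; FDestroyCheck destroys the actor unconditionally and prints a debug string.
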(event Custom|e_MarkSquare
  (Variables|Default|SetDestroy true))

(event EventBeginPlay)

(event Collision|EventActorBeginOverlap
  (params (OtherActor :type Actor%20Object%20Reference)))

(event EventTick
  (params (DeltaSeconds :type Float%20%28single-precision%29))
  (bind _cube (Variables|Default|GetCube))
  (bind _returnvalue (Transformation|GetWorldScale _cube))
  (bind _returnvalue_2 (- _returnvalue 0.01))
  (if (Variables|Default|GetEncroachment)
    (Transformation|SetWorldScale3D _cube (Math|Vector|MakeVector (.x _returnvalue_2) (.y _returnvalue_2) 1.0))
    (if (< (.x (Transformation|GetWorldScale _cube)) 0.01)
      (Actor|DestroyActor))))

(fn ConstructionScript)

(fn FDestroyCheck
  (Actor|DestroyActor)
  (Development|PrintString "REMOVE")
  (return))