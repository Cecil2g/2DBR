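; Player character for an archery game with a Paper2D sprite, moved on the X/Y plane by held-input flags from BP_PlayerController.
; An Idle/Drawing/Scouting state gates bow events and halves movement while drawing; Tick advances draw time and cooldown.
; Releasing spawns a BP_Arrow toward AimTarget with draw-scaled damage, and arrow overlaps reduce Health until destruction.
; Leaving all BP_AreaLimit volumes calls an empty environmental-death event, and scout camera logic is unwired.
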(event Custom|e_BeginDraw
  (if (and (> (Variables|Default|GetArrows) 0) (<= (Variables|Default|GetShotCooldown) 0.0))
    (Variables|Default|SetState "NewEnumerator1")))

(event Custom|e_BowFire
  (bind _state_match (CallFunction|FStateCheck true false true))
  (if _state_match
    (CallFunction|EBeginDraw)))

(event Custom|e_EndScout
  (params (Exit%20State :type E_PlayerState%20Enum :default "NewEnumerator0"))
  (Variables|Default|SetState Exit%20State)
  (CallFunction|FSquareRotation))

(event Custom|e_Collision
  (params (Actor :type Actor%20Object%20Reference))
  (bind _asbp_arrow (Utilities|Casting|CastToBP_Arrow Actor))
  (CallFunction|FCalcDamage _asbp_arrow))

(event Custom|e_EndDraw
  (params (Exit%20State :type E_PlayerState%20Enum :default "NewEnumerator0"))
  (Variables|Default|SetState Exit%20State)
  (Variables|Default|SetDrawTimer 0.0)
  (CallFunction|FSquareRotation))

(event Custom|e_BowRelease
  (bind _state_match (CallFunction|FStateCheck false true false))
  (if _state_match
    (CallFunction|FFireArrow)
    (CallFunction|EEndDraw "NewEnumerator0")))

(event Custom|e_BeginScout
  (bind _state_match (CallFunction|FStateCheck false true false))
  (if _state_match
    (CallFunction|EEndDraw "NewEnumerator2"))
  (Variables|Default|SetState "NewEnumerator2"))

(event Custom|e_EnviromentalDeath)

(event EventTick
  (params (DeltaSeconds :type Float%20%28single-precision%29))
  (Utilities|FlowControl|Sequence
    (:then_0
      ;[1 1 1] HandleMovement
      (CallFunction|FDirectionalMovement))
    (:then_1
      ;[1 1 1] Incriment DrawTimer
      (switch Utilities|FlowControl|Switch|SwitchonE_PlayerState (Variables|Default|GetState)
        (:NewEnumerator1
          (if (< (Variables|Default|GetDrawTimer) (Variables|Default|GetDrawTimerMax))
            (Variables|Default|SetDrawTimer (+ (Variables|Default|GetDrawTimer) DeltaSeconds))))))
    (:then_2
      ;[1 1 1] Decriment Shot cooldown
      (if (> (Variables|Default|GetShotCooldown) 0.0)
        (Variables|Default|SetShotCooldown (- (Variables|Default|GetShotCooldown) DeltaSeconds))))
    (:then_3
      ;[1 1 1] Draw line debug
      (switch Utilities|FlowControl|Switch|SwitchonE_PlayerState (Variables|Default|GetState)
        (:NewEnumerator1
          (Rendering|Debug|DrawDebugLine (Transformation|GetActorLocation) (Variables|Default|GetAimTarget) "(R=0.198794,G=1.000000,B=0.000000,A=1.000000)" 0.0 3.0))))
    (:then_4
      ;[1 1 1] Normalise camera
      (switch Utilities|FlowControl|Switch|SwitchonE_PlayerState (Variables|Default|GetState)
        (:NewEnumerator0
          (CallFunction|FNormaliseCamera))))))

(event Collision|EventActorEndOverlap
  (params (OtherActor :type Actor%20Object%20Reference))
  (CallFunction|FCheckBoundsWalkout OtherActor))

(event Collision|EventActorBeginOverlap
  (params (OtherActor :type Actor%20Object%20Reference))
  (CallFunction|ECollision OtherActor))

(fn ConstructionScript)

(fn FDirectionalMovement
  (bind (_asbp_player_controller _bsuccess) (CallFunction|FGetPlayerController))
  (bind _local_stop (LocalVariables|Getlocal_Stop))
  (if _bsuccess
    (bind _state_match (CallFunction|FStateCheck false true false))
    (if _state_match
      (LocalVariables|Setlocal_SpeedMod 0.5))
    (bind _output_get (LocalVariables|Setlocal_Speed (* (LocalVariables|Getlocal_SpeedMod) (Variables|Default|GetBaseSpeed))))
    (if (Variables|/Game/Core/BP_PlayerController.BP_PlayerController_C|GetRight%20Held _asbp_player_controller)
      (Pawn|Input|AddMovementInput (Math|Vector|MakeVector _output_get 0.0 0.0) 1.0 false)
      (else
        (Math|Integer|IncrementInt _local_stop
          (:%20%20
            _))))
    (if (Variables|/Game/Core/BP_PlayerController.BP_PlayerController_C|GetLeft%20Held _asbp_player_controller)
      (Pawn|Input|AddMovementInput (Math|Vector|MakeVector (* _output_get -1.0) 0.0 0.0) 1.0 false)
      (else
        (Math|Integer|IncrementInt _local_stop
          (:%20%20
            _))))
    (if (Variables|/Game/Core/BP_PlayerController.BP_PlayerController_C|GetUp%20Held _asbp_player_controller)
      (Pawn|Input|AddMovementInput (Math|Vector|MakeVector 0.0 (* _output_get -1.0) 0.0) 1.0 false)
      (else
        (Math|Integer|IncrementInt _local_stop
          (:%20%20
            _))))
    (if (Variables|/Game/Core/BP_PlayerController.BP_PlayerController_C|GetDown%20Held _asbp_player_controller)
      (Pawn|Input|AddMovementInput (Math|Vector|MakeVector 0.0 _output_get 0.0) 1.0 false)
      (else
        (Math|Integer|IncrementInt _local_stop
          (:%20%20
            _))))
    (if (== (LocalVariables|Getlocal_Stop) 4)
      (Variables|/Script/Engine.MovementComponent|SetVelocity (Variables|Character|GetCharacterMovement) "0, 0, 0"))
    (return)))

(fn FStateCheck
  (params (Idle :type Boolean) (Drawing :type Boolean) (Scouting :type Boolean))
  (bind _state (Variables|Default|GetState))
  (if Idle
    (if (Utilities|Enum|Equal(Enum) _state "NewEnumerator0")
      _
      (else
        (if Drawing :!label _label
          (if (Utilities|Enum|Equal(Enum) _state "NewEnumerator1")
            _
            (else
              (if Scouting :!label _label_2
                (if (Utilities|Enum|Equal(Enum) _state "NewEnumerator2")
                  _
                  (else
                    (return false)))
                (else
                  (return false)))))
          (else
            (goto _label_2)))))
    (else
      (goto _label)))
  (return true))

(fn FFireArrow
  (bind _returnvalue (Transformation|GetActorLocation))
  (bind _self self)
  (bind _returnvalue_2 (Game|SpawnActorfromClass "/Game/Core/BP_Arrow.BP_Arrow_C" (Math|Transform|MakeTransform _returnvalue (Math|Rotator|FindLookatRotation _returnvalue (Variables|Default|GetAimTarget)) "1,1,1") "AlwaysSpawn" _self _self))
  (bind _output_get (Variables|/Game/Core/BP_Arrow.BP_Arrow_C|SetDamage _returnvalue_2 (+ 2e+01 (/ (Variables|Default|GetDrawTimer) 3.0))))
  (Development|PrintString (Utilities|String|ToString(Float) _output_get) true true "(R=0.190345,G=1.000000,B=0.000000,A=1.000000)")
  (Math|Integer|DecrementInt (Variables|Default|GetArrows)
    (:%20%20
      (Variables|Default|SetShotCooldown (Variables|Default|GetShotCooldownMax))
      (return))))

(fn FSquareRotation
  (Transformation|SetWorldRotation (Variables|Default|GetPaperSprite) (Math|Rotator|MakeRotator 9e+01 0.0 0.0) false false))

(fn FCalcDamage
  (params (Arrow%20In :type BP%20Arrow%20Object%20Reference))
  (if (== (Variables|/Script/Engine.Actor|GetInstigator Arrow%20In) (Game|GetInstigator))
    (Development|PrintString "SEFL FIRE"))
  (Variables|Default|SetHealth (- (Variables|Default|GetHealth) (Variables|/Game/Core/BP_Arrow.BP_Arrow_C|GetDamage Arrow%20In)))
  (if (<= (Variables|Default|GetHealth) 0.0)
    (CallFunction|FKillPlayer))
  (return))

(fn FKillPlayer
  (Actor|DestroyActor)
  (return))

(fn FScout
  (Transformation|SetWorldLocation (Variables|Default|GetCamera) (+ (Transformation|GetActorLocation) (* (Variables|/Game/Core/BP_PlayerController.BP_PlayerController_C|GetAimTarget (.AsBP%20Player%20Controller (CallFunction|FGetPlayerController))) 0.1)) false false))

(fn FNormaliseCamera
  (Transformation|SetWorldLocation (Variables|Default|GetCamera) (Transformation|GetWorldLocation (Variables|Default|GetSprite)) false false))

(fn FCheckBoundsWalkout
  (params (Object :type Object%20Object%20Reference))
  (Utilities|Casting|CastToBP_AreaLimit Object)
  (for _array_element (Collision|GetOverlappingActors "/Game/Core/BP_AreaLimit.BP_AreaLimit_C" :!class /Script/Engine.Actor)
    (Utilities|Casting|CastToBP_AreaLimit _array_element)
    (LocalVariables|SetLocal_Safe true))
  (if (not (LocalVariables|GetLocal_Safe))
    (CallFunction|EEnviromentalDeath)))

(fn FCheckBoundsRestriction
  (for _array_element (Collision|GetOverlappingActors "/Game/Core/BP_AreaLimit.BP_AreaLimit_C" :!class /Script/Engine.Actor)
    (Utilities|Casting|CastToBP_AreaLimit _array_element)
    (LocalVariables|SetLocal_Safe true)
    (Development|PrintString "RESTRICT"))
  (if (not (LocalVariables|GetLocal_Safe))
    (CallFunction|EEnviromentalDeath)))

(fn FGetPlayerController
  (bind _returnvalue (Pawn|GetController))
  (bind (_asbp_player_controller _bsuccess) (Utilities|Casting|CastToBP_PlayerController _returnvalue))
  (return _asbp_player_controller _bsuccess))