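; BP_Torch is a torch actor that arrows can light or put out.
; On overlap with a BP_Arrow, a Fire effect lights an unlit torch and an Ice effect extinguishes a lit one.
; The light and extinguish events set Lit, which has an empty OnRep, and toggle TorchLight visibility.
; Extinguishing also zeroes the light intensity, which lighting never restores, and prints a debug string.
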(event Custom|e_LightTorch
  (Variables|Default|SetLit true)
  (Rendering|SetVisibility (Variables|Default|GetTorchLight) true true))

(event Custom|e_ExtinguishTorch
  (bind _torchlight (Variables|Default|GetTorchLight))
  (Variables|Default|SetLit false)
  (Rendering|SetVisibility _torchlight false true)
  (Rendering|Components|Light|SetIntensity _torchlight 0.0)
  (Development|PrintString "999999999999999999" true true "(R=1.000000,G=0.000000,B=0.172361,A=1.000000)" 4e+01))

(event EventBeginPlay)

(event Collision|EventActorBeginOverlap
  (params (OtherActor :type Actor%20Object%20Reference))
  (bind (_asbp_arrow _bsuccess) (Utilities|Casting|CastToBP_Arrow OtherActor))
  (bind _lit (Variables|Default|GetLit))
  (bind _arrowdata (Variables|/Game/Core/BP_Arrow.BP_Arrow_C|GetArrowData _asbp_arrow))
  (if _bsuccess
    (if (Utilities|Name|Equal(Name) (.effect _arrowdata) "Fire")
      (if (not _lit)
        (CallFunction|ELightTorch))
      (elif (Utilities|Name|Equal(Name) (.effect _arrowdata) "Ice")
        (if _lit
          (CallFunction|EExtinguishTorch))))))

(event EventTick
  (params (DeltaSeconds :type Float%20%28single-precision%29)))

(fn ConstructionScript)

(fn OnRepLit)