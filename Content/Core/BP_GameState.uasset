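; Game state that runs a server-driven shrinking play area, battle-royale style, over 16 data-table-placed BP_AreaLimit squares.
; A per-tick countdown destroys marked squares and advances the phase, refreshing player minimaps.
; Phases 1–4 place a BP_AreaSelector beside the squares' average location, randomizing sides and alternating axes within each pair; phase 5 starts encroachment instead.
; Arrow and global-message handlers are stubs, with old logic left disconnected.
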(event Custom|e_BeginPlay
  (for _index (range 1 16)
    (AreaRestriction|FSpawnSquare _index))
  (AreaRestriction|FMakeMinimap)
  (CallFunction|EPhaseIncrement))

(event Custom|e_PhaseIncrement
  (Networking|SwitchHasAuthority
    (:Authority
      (bind _returnvalue (Game|SpawnActorfromClass "/Game/Core/BP_AreaSelector.BP_AreaSelector_C" (Math|Transform|MakeTransform "0, 0, 0" "0, 0, 0" "1.000000,1.000000,0.600000") "Undefined" 0 0))
      (bind _result (Math|Integer|IncrementInt (Variables|Default|GetPhase))
        (:%20%20
          (AreaRestriction|FResizeGameArea _result _returnvalue)
          (Utilities|IsValid _returnvalue
            (:Is%20Valid
              (Default|ESpawnSequence _returnvalue _result))
            (:Is%20Not%20Valid
              _))
          (CallFunction|ERefreshMinimaps)
          (CallFunction|EGlobalMessage "LALALALLALALALA"))))))

(event Custom|e_RefreshMinimaps
  (Networking|SwitchHasAuthority
    (:Authority
      (bind _outactors (Actor|GetAllActorsOfClass "/Game/Core/BP_PlayerController.BP_PlayerController_C"))
      (Development|PrintString (Utilities|String|ToString(Integer) (Utilities|Array|Length _outactors)) true true "(R=0.576999,G=1.000000,B=0.000000,A=1.000000)" 6e+01)
      (for _array_element _outactors
        (Default|ERefreshUI _array_element)))))

(event Custom|e_GlobalMessage
  (params (Message%20In :type Text))
  (Networking|SwitchHasAuthority
    (:Authority
      (CallFunction|FGlobalMessage Message%20In))))

(event Custom|e_GS_ArrowFire
  (params (Launcher :type BP%20Player%20Character%20Object%20Reference))
  (CallFunction|EGSArrowFireMulti Launcher))

(event Custom|e_GS_ArrowHit)

(event Custom|e_DestroyMarked
  (bind _arealimits (Variables|Default|GetAreaLimits))
  (bind (_arrayindex _arrayelement) (Utilities|Array|ReverseforEachLoop _arealimits)
    (:LoopBody
      (if (Variables|/Game/Core/BP_AreaLimit.BP_AreaLimit_C|GetDestroy _arrayelement)
        (Default|FDestroyCheck _arrayelement)
        (Utilities|Array|RemoveIndex _arealimits _arrayindex)))))

(event Custom|e_GS_ArrowFireMulti
  (params (Launcher :type BP%20Player%20Character%20Object%20Reference)))

(event EventBeginPlay
  (Networking|SwitchHasAuthority
    (:Authority
      (CallFunction|EBeginPlay))))

(event EventTick
  (params (DeltaSeconds :type Float%20%28single-precision%29))
  (Networking|SwitchHasAuthority
    (:Authority
      (bind _outactors (Actor|GetAllActorsOfClass "/Game/Core/BP_PlayerController.BP_PlayerController_C"))
      (Development|PrintString (Utilities|String|ToString(Integer) (Utilities|Array|Length _outactors)) true true "(R=1.000000,G=0.573006,B=0.000000,A=1.000000)" 0.0)
      (Development|PrintString (Utilities|String|ToString(Integer) (Variables|Default|GetPhaseTimer)) true true "(R=1.000000,G=0.000000,B=0.390983,A=1.000000)" 0.0)
      (Math|Integer|DecrementInt (Variables|Default|GetPhaseTimer)
        (:%20%20
          (if (== (Variables|Default|GetPhaseTimer) 0)
            (CallFunction|EDestroyMarked)
            (CallFunction|EPhaseIncrement)))))))

(fn ConstructionScript)

(fn FSpawnSquare
  (params (Ref%20In :type Integer))
  (bind _gridsize (Variables|Default|GetGridSize))
  (bind _returnvalue (Utilities|GetDataTableRow "/Game/Core/DT_AreaLimitData.DT_AreaLimitData" (Utilities|String|StringToName (Utilities|String|ToString(Integer) Ref%20In)))
    (:then
      (bind _returnvalue_2 (Game|SpawnActorfromClass "/Game/Core/BP_AreaLimit.BP_AreaLimit_C" (Math|Transform|MakeTransform (+ (Math|Vector|MakeVector (* (.xoffset _returnvalue) _gridsize) (* (.yoffset _returnvalue) _gridsize) 0.0) (Math|Vector|MakeVector 0.0 0.0 0.0)) "0, 0, 0" "1,1,1") "Undefined" 0 0))
      (Transformation|SetActorLocation _returnvalue_2 (Math|Vector|MakeVector (- (.x (Transformation|GetActorLocation _returnvalue_2)) 8.0) (- (.y (Transformation|GetActorLocation _returnvalue_2)) 8.0) (.z (Transformation|GetActorLocation _returnvalue_2))) false false)
      (Utilities|Array|Add (Variables|Default|GetAreaLimits) _returnvalue_2))
    (:RowNotFound
      (Development|PrintString "DT NOT FOUND"))))

(fn FMakeMinimap
  (bind _outactors (Actor|GetAllActorsOfClass "/Game/Core/BP_PlayerController.BP_PlayerController_C"))
  (for _array_element _outactors
    (Default|EMakeGridSquares (Variables|/Game/UI/UI_HUD.UI_HUD_C|GetUI_Minimap (Variables|/Game/Core/BP_PlayerController.BP_PlayerController_C|GetHUD _array_element)))))

(fn FPhaseIncrement)

(fn FResizeGameArea
  (params (Phase%20In :type Integer) (Area%20Selector%20In :type Actor%20Object%20Reference))
  (switch int Phase%20In
    (:1
      (Variables|Default|SetPhaseTimer 600)
      (bind (_location_out _scale_out) (AreaRestriction|FResize1 1024.0))
      (Transformation|SetActorTransform Area%20Selector%20In (Math|Transform|MakeTransform _location_out "0, 0, 0" _scale_out))
      (return))
    (:2
      (Variables|Default|SetPhaseTimer 600)
      (bind (_location_out_2 _scale_out_2) (AreaRestriction|FResize2))
      (Transformation|SetActorTransform Area%20Selector%20In (Math|Transform|MakeTransform _location_out_2 "0, 0, 0" _scale_out_2))
      (bind _outactors (Actor|GetAllActorsOfClass "/Game/Core/BP_PlayerController.BP_PlayerController_C" :!label _label))
      (for _array_element _outactors
        (Utilities|IsValid (.AsBP%20Player%20Character (Utilities|Casting|CastToBP_PlayerCharacter (Pawn|GetControlledPawn _array_element)))
          (:Is%20Valid
            (Default|FCheckBoundsRestriction (.AsBP%20Player%20Character (Utilities|Casting|CastToBP_PlayerCharacter (Pawn|GetControlledPawn _array_element)))))
          (:Is%20Not%20Valid
            (Development|PrintString "NOTVALID"))))
      (return))
    (:3
      (Variables|Default|SetPhaseTimer 300)
      (bind (_location_out_3 _scale_out_3) (AreaRestriction|FResize3 768.0))
      (Transformation|SetActorTransform Area%20Selector%20In (Math|Transform|MakeTransform _location_out_3 "0, 0, 0" _scale_out_3))
      (goto _label))
    (:4
      (Variables|Default|SetPhaseTimer 300)
      (bind (_location_out_4 _scale_out_4) (AreaRestriction|FResize4))
      (Transformation|SetActorTransform Area%20Selector%20In (Math|Transform|MakeTransform _location_out_4 "0, 0, 0" _scale_out_4))
      (goto _label))
    (:5
      (Actor|DestroyActor Area%20Selector%20In)
      (Variables|/Game/Core/BP_AreaLimit.BP_AreaLimit_C|SetEncroachment (Utilities|Array|Get(acopy) (Variables|Default|GetAreaLimits)) true))))

(fn FResize1
  (params (Dimension%20In :type Float%20%28single-precision%29))
  (bind _averagevector_out (AreaRestriction|FGetAverageLocation))
  (LocalVariables|SetDimension Dimension%20In)
  (switch int (Math|Random|RandomIntegerinRange 1 4)
    (:1
      (LocalVariables|SetLocal%20Vector (Math|Vector|MakeVector (+ (.x _averagevector_out) (LocalVariables|GetDimension)) (.y _averagevector_out) 0.0))
      (LocalVariables|SetLocal%20Scale "1.500000,3.500000,1.000000" :!label _label)
      (Variables|Default|SetLast%20Reduction "NewEnumerator1"))
    (:2
      (LocalVariables|SetLocal%20Vector (Math|Vector|MakeVector (- (.x _averagevector_out) (LocalVariables|GetDimension)) (.y _averagevector_out) 0.0))
      (goto _label))
    (:3
      (LocalVariables|SetLocal%20Vector (Math|Vector|MakeVector (.x _averagevector_out) (+ (.y _averagevector_out) (LocalVariables|GetDimension)) 0.0))
      (LocalVariables|SetLocal%20Scale "3.500000,1.500000,1.000000" :!label _label_2)
      (Variables|Default|SetLast%20Reduction "NewEnumerator0"))
    (:4
      (LocalVariables|SetLocal%20Vector (Math|Vector|MakeVector (.x _averagevector_out) (- (.y _averagevector_out) (LocalVariables|GetDimension)) 0.0))
      (goto _label_2)))
  (return (LocalVariables|GetLocal%20Vector) (LocalVariables|GetLocal%20Scale)))

(fn FGetAverageLocation
  (bind _arealimits (Variables|Default|GetAreaLimits))
  (Development|PrintString (Utilities|String|ToString(Integer) (Utilities|Array|Length _arealimits)))
  (for _array_element _arealimits
    (LocalVariables|SetAverageVector (+ (Transformation|GetActorLocation _array_element) (LocalVariables|GetAverageVector)))
    (Math|Integer|IncrementInt (LocalVariables|GetAreaCount)))
  (return (/ (LocalVariables|GetAverageVector) (LocalVariables|GetAreaCount))))

(fn FResize2
  (bind _returnvalue (Math|Random|RandomIntegerinRange 1 2))
  (bind _averagevector_out (AreaRestriction|FGetAverageLocation))
  (bind _dimension (LocalVariables|GetDimension))
  (switch Utilities|FlowControl|Switch|SwitchonE_ReductionTypes (Variables|Default|GetLast%20Reduction)
    (:NewEnumerator0
      (switch int _returnvalue
        (:1
          (LocalVariables|SetLocal%20Vector (Math|Vector|MakeVector (+ (.x _averagevector_out) _dimension) (.y _averagevector_out) 0.0)))
        (:2
          (LocalVariables|SetLocal%20Vector (Math|Vector|MakeVector (- (.x _averagevector_out) _dimension) (.y _averagevector_out) 0.0))))
      (LocalVariables|SetLocal%20Scale "1.000000,1.000000,1.000000"))
    (:NewEnumerator1
      (switch int _returnvalue
        (:1
          (LocalVariables|SetLocal%20Vector (Math|Vector|MakeVector (.x _averagevector_out) (+ (.y _averagevector_out) _dimension) 0.0)))
        (:2
          (LocalVariables|SetLocal%20Vector (Math|Vector|MakeVector (.x _averagevector_out) (- (.y _averagevector_out) _dimension) 0.0))))
      (LocalVariables|SetLocal%20Scale "1.000000,1.000000,1.000000")))
  (return (LocalVariables|GetLocal%20Vector) (LocalVariables|GetLocal%20Scale)))

(fn FResize3
  (params (Dimension%20In :type Float%20%28single-precision%29))
  (bind _averagevector_out (AreaRestriction|FGetAverageLocation))
  (LocalVariables|SetDimension Dimension%20In)
  (switch int (Math|Random|RandomIntegerinRange 1 4)
    (:1
      (LocalVariables|SetLocal%20Vector (Math|Vector|MakeVector (+ (.x _averagevector_out) (LocalVariables|GetDimension)) (.y _averagevector_out) 0.0))
      (LocalVariables|SetLocal%20Scale "1.000000,1.000000,1.000000" :!label _label)
      (Variables|Default|SetLast%20Reduction "NewEnumerator1"))
    (:2
      (LocalVariables|SetLocal%20Vector (Math|Vector|MakeVector (- (.x _averagevector_out) (LocalVariables|GetDimension)) (.y _averagevector_out) 0.0))
      (goto _label))
    (:3
      (LocalVariables|SetLocal%20Vector (Math|Vector|MakeVector (.x _averagevector_out) (+ (.y _averagevector_out) (LocalVariables|GetDimension)) 0.0))
      (LocalVariables|SetLocal%20Scale "1.000000,1.000000,1.000000" :!label _label_2)
      (Variables|Default|SetLast%20Reduction "NewEnumerator0"))
    (:4
      (LocalVariables|SetLocal%20Vector (Math|Vector|MakeVector (.x _averagevector_out) (- (.y _averagevector_out) (LocalVariables|GetDimension)) 0.0))
      (goto _label_2)))
  (return (LocalVariables|GetLocal%20Vector) (LocalVariables|GetLocal%20Scale)))

(fn FResize4
  (bind _returnvalue (Math|Random|RandomIntegerinRange 1 2))
  (bind _averagevector_out (AreaRestriction|FGetAverageLocation))
  (bind _dimension (LocalVariables|GetDimension))
  (switch Utilities|FlowControl|Switch|SwitchonE_ReductionTypes (Variables|Default|GetLast%20Reduction)
    (:NewEnumerator0
      (switch int _returnvalue
        (:1
          (LocalVariables|SetLocal%20Vector (Math|Vector|MakeVector (+ (.x _averagevector_out) _dimension) (.y _averagevector_out) 0.0)))
        (:2
          (LocalVariables|SetLocal%20Vector (Math|Vector|MakeVector (- (.x _averagevector_out) _dimension) (.y _averagevector_out) 0.0))))
      (LocalVariables|SetLocal%20Scale "0.500000,0.500000,1.000000"))
    (:NewEnumerator1
      (switch int _returnvalue
        (:1
          (LocalVariables|SetLocal%20Vector (Math|Vector|MakeVector (.x _averagevector_out) (+ (.y _averagevector_out) _dimension) 0.0)))
        (:2
          (LocalVariables|SetLocal%20Vector (Math|Vector|MakeVector (.x _averagevector_out) (- (.y _averagevector_out) _dimension) 0.0))))
      (LocalVariables|SetLocal%20Scale "0.500000,0.500000,1.000000")))
  (return (LocalVariables|GetLocal%20Vector) (LocalVariables|GetLocal%20Scale)))

(fn FGlobalMessage
  (params (Message%20In :type Text)))